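; BP_Allumette is a match ("allumette") pickup item that the player collects by interacting with it.
; On BeginPlay it caches the BP_Player reference and applies an outline overlay material to its Cube mesh.
; Interact sets HasAllumette on the cached player, posts a pickup notification through the interacting player's HUD, then destroys only the Cube component.
; BPGetItemName supplies the item name and prompt visibility.
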(event `self.ReceiveBeginPlay`
  ;[0.05098 0.05098 0.05098] Cast to Player
  (bind _asbp_player (cast `/Game/FPMovement/Player/Blueprints/BP_Player` (`GameplayStatics.GetPlayerCharacter` 0)))
  (set `self.Player Reference` _asbp_player)
  (`MeshComponent.SetOverlayMaterial` (`self.Cube`) "/Game/Jarir/Outline/Mi_SimpleOutline1_Inst.Mi_SimpleOutline1_Inst"))

(event `self.BP_Interact`
  (params (FPMovementPlayer :type "/Game/FPMovement/Player/Blueprints/BP_Player Object Reference"))
  ;[0.05098 0.05098 0.05098] Pickup/Destroy function
  (set `/Game/FPMovement/Player/Blueprints/BP_Player.HasAllumette?` true (`self.Player Reference`))
  (`/Game/Jarir/UI/WB_PlayerHud.AddNotification` (`/Game/FPMovement/Player/Blueprints/BP_Player.Hud Reference` FPMovementPlayer) (`self.Pickup Notification`) (`KismetTextLibrary.Conv_NameToText` (`self.Item Name`)) (`self.Item Color Notification`))
  (if true
    (`ActorComponent.K2_DestroyComponent` (`self.Cube`))))

(fn `BP_GetItemName`
  (returns (ItemName :type Name) (`ShowItemPromt?` :type Boolean))
  (return (`self.Item Name`) (`self.Show Item Prompt?`)))

(fn `UserConstructionScript`)