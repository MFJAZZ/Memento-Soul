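; BP_Cheminée is an interactable fireplace that the player lights with a match (allumette).
; Overlapping its Box shows a WB_InteractDot widget, removed when the player leaves.
; Interact checks the player's HasAllumette flag, printing a message if false; otherwise it spawns Feu in place and updates the mission to opening the barricaded door.
; It then disables input, shows the cursor and a dialogue widget, and destroys itself.
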(event `self.ReceiveBeginPlay`
  (bind _asbp_player (cast `/Game/FPMovement/Player/Blueprints/BP_Player` (`GameplayStatics.GetPlayerCharacter` 0)))
  (set `self.As BP Player` _asbp_player))

(event `/Game/FPMovement/Player/Blueprints/Interface/BP_Interact.BP_Interact`
  (params (FPMovementPlayer :type "/Game/FPMovement/Player/Blueprints/BP_Player Object Reference"))
  (if (`/Game/FPMovement/Player/Blueprints/BP_Player.HasAllumette?` (`self.As BP Player`))
    (if true
      (`|SpawnActorFromClass` "/Game/Jarir/Vie/Feu.Feu_C" (`self.GetTransform`) "Undefined" "MultiplyWithRoot" null null)
      (`/Game/FPMovement/Player/Blueprints/BP_Player.UpdateMission` (`self.As BP Player`) "Trouvez un moyen d'ouvrir la porte barricadé")
      (`/Engine/EditorBlueprintResources/StandardMacros.DoOnce` false
        (:`Completed`
          (`self.DisableInput` (`GameplayStatics.GetPlayerCharacter` 0) null)
          (set `PlayerController.bShowMouseCursor` true (`GameplayStatics.GetPlayerController` 0))
          (bind _returnvalue (`|CreateWidget` "/Game/Jarir/Dialogues/HUD/HUD_Dialogu2.HUD_Dialogu2_C"))
          (`UserWidget.AddToViewport` _returnvalue 0)
          (`self.K2_DestroyActor`))))
    (else
      (`KismetSystemLibrary.PrintString` "Aucune Allumette"))))

(event `self.Box.OnComponentBeginOverlap`
  (params (OverlappedComponent :type "PrimitiveComponent Object Reference") (OtherActor :type "Actor Object Reference") (OtherComp :type "PrimitiveComponent Object Reference") (OtherBodyIndex :type Integer) (bFromSweep :type Boolean) (SweepResult :type "HitResult Structure (by ref)"))
  (if (== OtherActor (`GameplayStatics.GetPlayerPawn` 0))
    (`/Engine/EditorBlueprintResources/StandardMacros.DoOnce` false :!label _label
      (:`Completed`
        (bind _returnvalue (`|CreateWidget` "/Game/idris/couloir/porte/BP_porte/WB_InteractDot.WB_InteractDot_C"))
        (`UserWidget.AddToViewport` _returnvalue 0)))))

(event `self.Box.OnComponentEndOverlap`
  (params (OverlappedComponent :type "PrimitiveComponent Object Reference") (OtherActor :type "Actor Object Reference") (OtherComp :type "PrimitiveComponent Object Reference") (OtherBodyIndex :type Integer))
  (if (== OtherActor (`GameplayStatics.GetPlayerPawn` 0))
    (`/Game/idris/couloir/porte/BP_porte/WB_InteractDot.RemoveDot` (stale `self.Box.OnComponentBeginOverlap` _returnvalue))
    (goto _label :!via `Reset`)))

(fn `UserConstructionScript`)