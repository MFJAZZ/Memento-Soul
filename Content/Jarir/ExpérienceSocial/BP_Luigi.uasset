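; BP_Luigi is an interactable actor that plays a 2D sound (Darksoul__1_) and destroys itself when Interact is triggered.
; When the player pawn enters its Box, it creates a WB_InteractDot widget and adds it to the viewport as a prompt.
; A DoOnce prevents duplicate dots; leaving the Box calls RemoveDot on the widget and resets the gate.
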(event `/Game/FPMovement/Player/Blueprints/Interface/BP_Interact.BP_Interact`
  (params (FPMovementPlayer :type "/Game/FPMovement/Player/Blueprints/BP_Player Object Reference"))
  (`GameplayStatics.PlaySound2D` "/Game/Jarir/Sounds/dark-soul__1_.dark-soul__1_" 0.7 1.0 0.0 null null)
  (`self.K2_DestroyActor`))

(event `self.Box.OnComponentBeginOverlap`
  (params (OverlappedComponent :type "PrimitiveComponent Object Reference") (OtherActor :type "Actor Object Reference") (OtherComp :type "PrimitiveComponent Object Reference") (OtherBodyIndex :type Integer) (bFromSweep :type Boolean) (SweepResult :type "HitResult Structure (by ref)"))
  (if (== OtherActor (`GameplayStatics.GetPlayerPawn` 0))
    (`/Engine/EditorBlueprintResources/StandardMacros.DoOnce` false :!label _label
      (:`Completed`
        (bind _returnvalue (`|CreateWidget` "/Game/idris/couloir/porte/BP_porte/WB_InteractDot.WB_InteractDot_C"))
        (`UserWidget.AddToViewport` _returnvalue 0)))))

(event `self.Box.OnComponentEndOverlap`
  (params (OverlappedComponent :type "PrimitiveComponent Object Reference") (OtherActor :type "Actor Object Reference") (OtherComp :type "PrimitiveComponent Object Reference") (OtherBodyIndex :type Integer))
  (if (== OtherActor (`GameplayStatics.GetPlayerPawn` 0))
    (`/Game/idris/couloir/porte/BP_porte/WB_InteractDot.RemoveDot` (stale `self.Box.OnComponentBeginOverlap` _returnvalue))
    (goto _label :!via `Reset`)))

(fn `UserConstructionScript`)