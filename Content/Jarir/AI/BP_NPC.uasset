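; BP_NPC is a hostile NPC that opens doors in its way and jumpscares the player on contact.
; Its DoorCollider calls DoorTest on any closed BP_BaseDoor it overlaps.
; A Box overlap with BP_Player triggers the jumpscare, disables input and plays a zombie attack animation, then after a delay pauses the game and shows the DeathScreen widget with the cursor.
; The owner door reference cached on BeginPlay is unused.
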(event `self.ReceiveBeginPlay`
  (bind _asbp_base_door (cast `/Game/Jarir/Door/BP_BaseDoor` (`self.GetOwner`)))
  (set `self.As Door ref` _asbp_base_door))

(event `self.DoorCollider.OnComponentBeginOverlap`
  (params (OverlappedComponent :type "PrimitiveComponent Object Reference") (OtherActor :type "Actor Object Reference") (OtherComp :type "PrimitiveComponent Object Reference") (OtherBodyIndex :type Integer) (bFromSweep :type Boolean) (SweepResult :type "HitResult Structure (by ref)"))
  (bind _asbp_base_door (cast `/Game/Jarir/Door/BP_BaseDoor` OtherActor))
  (if (`/Game/Jarir/Door/BP_BaseDoor.IsClosed` _asbp_base_door)
    (`/Game/Jarir/Door/BP_BaseDoor.DoorTest` _asbp_base_door)
    (`KismetSystemLibrary.PrintString` "open da door")))

(event `self.Box.OnComponentBeginOverlap`
  (params (OverlappedComponent :type "PrimitiveComponent Object Reference") (OtherActor :type "Actor Object Reference") (OtherComp :type "PrimitiveComponent Object Reference") (OtherBodyIndex :type Integer) (bFromSweep :type Boolean) (SweepResult :type "HitResult Structure (by ref)"))
  ; Jumpscare
  (bind _asbp_player (cast `/Game/FPMovement/Player/Blueprints/BP_Player` OtherActor))
  (`/Game/FPMovement/Player/Blueprints/BP_Player.Jumpscare` _asbp_player)
  (`self.DisableInput` _asbp_player null)
  (`SkeletalMeshComponent.PlayAnimation` (`self.Mesh`) "/Game/Jarir/AI/Anime/ZombieAttack_UE.ZombieAttack_UE" false)
  (`KismetSystemLibrary.Delay` 3.0)
  (`GameplayStatics.SetGamePaused` true)
  (set `PlayerController.bShowMouseCursor` true (`PlayerState.GetPlayerController` (`Pawn.PlayerState` _asbp_player)))
  (bind _returnvalue (`|CreateWidget` "/Game/Jarir/UI/DeathScreen.DeathScreen_C"))
  (`UserWidget.AddToViewport` _returnvalue 0))

(fn `UserConstructionScript`)